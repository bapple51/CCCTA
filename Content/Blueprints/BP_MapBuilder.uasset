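; BP_MapBuilder turns a queued address into the world's georeferenced origin, with an address input widget shown at BeginPlay.
; Tick polls RequestQueued and sends PendingAddress to OpenStreetMap's Nominatim search over HTTP GET.
; HandleGeocode strips the response's array brackets, parses lat/lon from the JSON, applies them to the GeoReferencing system at zero altitude, and prints a self-check conversion or failure message.
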(event `self.ReceiveBeginPlay`
  (bind _returnvalue (`GameplayStatics.GetPlayerController` 0))
  (set `PlayerController.bShowMouseCursor` true _returnvalue)
  (bind _returnvalue_2 (`|CreateWidget` "/Game/UI/WBP_AddressInput.WBP_AddressInput_C" _returnvalue))
  (`UserWidget.AddToViewport` _returnvalue_2 0))

(event `OnRequestComplete_Event`
  (params (Response :type String) (bSuccessful :type Boolean) (OutHeader :type "HttpHeader Structure"))
  (`self.HandleGeocode` Response bSuccessful))

(event `OnRequestComplete_Event_2`
  (params (Response :type String) (bSuccessful :type Boolean) (OutHeader :type "HttpHeader Structure")))

(event `OnRequestComplete_Event_3`
  (params (Response :type String) (bSuccessful :type Boolean) (OutHeader :type "HttpHeader Structure")))

(event `OnRequestComplete_Event_0`
  (params (Response :type String) (bSuccessful :type Boolean) (OutHeader :type "HttpHeader Structure")))

(event `self.ReceiveTick`
  (params (DeltaSeconds :type "Float (single-precision)"))
  (if (`self.bRequestQueued`)
    (set `self.bRequestQueued` false)
    (bind _returnvalue (`HttpRequestProxyObject.CreateHttpRequestProxyObject` (`KismetStringLibrary.Concat_StrStr` "https://nominatim.openstreetmap.org/search?format=json&limit=1&q=" (`KismetStringLibrary.Replace` (`self.PendingAddress`) " " "+")) "GET"))
    (add `HttpRequestProxyObject.OnRequestComplete` _returnvalue (delegate `OnRequestComplete_Event`))))

(event `GeoResp`)

(event `OnRequestComplete_Event_1`
  (params (Response :type String) (bSuccessful :type Boolean) (OutHeader :type "HttpHeader Structure")))

(event `GeoDone`)

(fn `HandleGeocode`
  (params (Response :type String) (bSuccessful :type Boolean))
  (bind _returnvalue (`GeoReferencingSystem.GetGeoReferencingSystem`))
  (if bSuccessful
    (bind (_outjsonobject _returnvalue_2) (`JsonBlueprintFunctionLibrary.FromString` (`KismetStringLibrary.LeftChop` (`KismetStringLibrary.RightChop` Response 1) 1)))
    (if _returnvalue_2
      (bind _outvalue (`|GetJsonField` _outjsonobject "lat"))
      (bind _outvalue_2 (`|GetJsonField` _outjsonobject "lon"))
      (bind _returnvalue_3 (`KismetStringLibrary.Conv_StringToDouble` _outvalue))
      (set `self.OriginLat` _returnvalue_3)
      (bind _returnvalue_4 (`KismetStringLibrary.Conv_StringToDouble` _outvalue_2))
      (set `self.OriginLon` _returnvalue_4)
      (set `GeoReferencingSystem.OriginLatitude` _returnvalue_3 _returnvalue)
      (set `GeoReferencingSystem.OriginLongitude` _returnvalue_4 _returnvalue)
      (set `GeoReferencingSystem.OriginAltitude` 0.0 _returnvalue)
      (`GeoReferencingSystem.ApplySettings` _returnvalue)
      (bind _enginecoordinates (`GeoReferencingSystem.GeographicToEngine` _returnvalue (`GeographicCoordinatesFunctionLibrary.MakeGeographicCoordinates` (`KismetMathLibrary.MakeVector` _returnvalue_3 _returnvalue_4))))
      (`KismetSystemLibrary.PrintString` (`KismetStringLibrary.Concat_StrStr` "ORIGIN SET selfcheck=" (`KismetStringLibrary.Conv_VectorToString` _enginecoordinates)) true true (struct :`G` 0.66 :`B` 1.0 :`A` 1.0) 30.0)
      (else
        (`KismetSystemLibrary.PrintString` "GEO json parse FAILED" true true (struct :`G` 0.66 :`B` 1.0 :`A` 1.0) 30.0)))
    (else
      (`KismetSystemLibrary.PrintString` "GEO request FAILED" true true (struct :`G` 0.66 :`B` 1.0 :`A` 1.0) 30.0))))

(fn `UserConstructionScript`)