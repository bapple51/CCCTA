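; HTTP probe actor that sets up a test GET request to OpenStreetMap's Nominatim geocoding search for Walnut Creek.
; BeginPlay creates the request proxy object with a hardcoded URL and binds its completion to an empty handler, so the response goes unused.
; A duplicate, unconnected chain binds the handler that would print a success or failure marker and the raw response, but it never runs.
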(event `self.ReceiveBeginPlay`
  (bind _returnvalue (`HttpRequestProxyObject.CreateHttpRequestProxyObject` "https://nominatim.openstreetmap.org/search?q=Walnut%20Creek&format=json&limit=1" "GET"))
  (add `HttpRequestProxyObject.OnRequestComplete` _returnvalue (delegate `OnRequestComplete_Event_1`)))

(event `CustomEvent`)

(event `OnRequestComplete_Event_0`
  (params (Response :type String) (bSuccessful :type Boolean) (OutHeader :type "HttpHeader Structure")))

(event `OnRequestComplete_Event`
  (params (Response :type String) (bSuccessful :type Boolean) (OutHeader :type "HttpHeader Structure"))
  (`KismetSystemLibrary.PrintString` (select `bool` bSuccessful :`false` "HTTPPROBE FAIL" :`true` "HTTPPROBE SUCCESS") true true (struct :`G` 0.66 :`B` 1.0 :`A` 1.0) 30.0)
  (`KismetSystemLibrary.PrintString` Response true true (struct :`G` 0.66 :`B` 1.0 :`A` 1.0) 30.0))

(event `OnRequestComplete_Event_1`
  (params (Response :type String) (bSuccessful :type Boolean) (OutHeader :type "HttpHeader Structure")))

(fn `UserConstructionScript`)